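; Bp_cazador is a hunter actor that moves and fires projectiles when a target is in range.
; A looping timer spawns Bp_Bala at the hunter's transform while EnRango is true, passing Objetivo as the projectile's target.
; Each Tick applies a scaled Objetivo as an unswept local offset, independent of delta time, and draws a large red debug sphere.
; Neither EnRango nor Objetivo is set within these graphs.
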(event Custom|shoot
  (if (Variables|Propiedades|Geten%20rango)
    (Game|SpawnActorfromClass "/Game/bp_Bala.bp_Bala_C" (Transformation|GetActorTransform) "Undefined" "MultiplyWithRoot" 0 (Variables|Propiedades|GetObjetivo) 0)))

(event EventTick
  (params (DeltaSeconds :type Float%20%28single-precision%29))
  (Transformation|AddActorLocalOffset (* (Variables|Propiedades|GetObjetivo) 1.2) false false)
  (Rendering|Debug|DrawDebugSphere (Transformation|GetActorLocation) 4e+03 36 "(R=1.000000,G=0.000000,B=0.000000,A=1.000000)" 0.1 5.0))

(event EventBeginPlay
  (Utilities|Time|SetTimerbyEvent (delegate Custom|shoot) 0.7 true))

(fn ConstructionScript)
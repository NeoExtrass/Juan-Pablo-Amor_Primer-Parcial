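; Prey actor that moves constantly along its local velocity direction and doubles its speed after being attacked.
; BeginPlay briefly draws a debug sphere marking the enemy spawn area, derives the doubled max speed and starts a looping timer polling the attacked flag.
; When flagged, it waits briefly, switches to fast movement and clears the timer.
; Tick applies normalized direction times current speed as an unswept local offset, without delta-time scaling.
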(event Custom|Atacado!
  ;[1 1 1] si es atacado, la velocidad se multiplica por 2
  (if (Variables|Propiedades|Getatacado?)
    (Utilities|FlowControl|Delay 1.0)
    (Variables|Propiedades|SetATACADO true)
    (Utilities|Time|ClearandInvalidateTimerbyHandle (stale EventBeginPlay _returnvalue))))

(event EventBeginPlay
  ;[1 1 1] marca el area inicial de aparicion de enemigos
  (Rendering|Debug|DrawDebugSphere (Transformation|GetActorLocation) 4e+03 36 "(R=1.000000,G=1.000000,B=1.000000,A=1.000000)" 3.0 2e+01)
  ;[1 1 1] se asigna la velocidad maxima a la que ira el personaje al ser atacado
  (Variables|Propiedades|SetMax%20speed (* (Variables|Propiedades|GetMultiplicador%20de%20velocidad) 2.0))
  (bind _returnvalue (Utilities|Time|SetTimerbyEvent (delegate Custom|Atacado!) 2.0 true)))

(event EventTick
  (params (DeltaSeconds :type Float%20%28single-precision%29))
  (if (Variables|Propiedades|GetATACADO)
    ;[1 1 1] la funcion determina la velocidad de movimiento
    (bind _returnvalue (CallFunction|SetMaxSpeed))
    (Transformation|AddActorLocalOffset _returnvalue false false)
    (else
      ;[1 1 1] la funcion determina la velocidad de movimiento
      (bind _returnvalue_2 (CallFunction|SetActorOffsetSpeed))
      (Transformation|AddActorLocalOffset _returnvalue_2 false false))))

(fn ConstructionScript)

(fn SetActorOffsetSpeed
  (return (* (Math|Vector|Normalize (Variables|Propiedades|GetVelocidad)) (Variables|Propiedades|GetMultiplicador%20de%20velocidad))))

(fn SetMaxSpeed
  (return (* (Math|Vector|Normalize (Variables|Propiedades|GetVelocidad)) (Variables|Propiedades|GetMax%20speed))))